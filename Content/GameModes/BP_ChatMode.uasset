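; Game mode for a turn-based two-player number baseball game played through chat between a Host and a Guest.
; It generates the secret number with a C++ library, broadcasts it and client messages to every BP_Controller, and advances turns.
; A C++ rule function scores guesses; a full-strike result prints the winner, both players exhausting their counts prints a draw, and either resets the round.
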(event Custom|GotTextCheck
  (params (Msg :type String))
  ;[0.15 0.15 0.15 0.5] 판정 로직 C++ 라이브 러리
  (bind _returnvalue (Class|BFBaseball|BaseBallRule Msg (Variables|Default|GetRandomNumber)))
  (CallFunction|GameWinnerCheck _returnvalue)
  (if (Variables|Default|GetEndFlag)
    (CallFunction|ResetGame)
    (else
      (bind _outactors (Actor|GetAllActorsOfClass "/Script/Engine.PlayerController"))
      (for _array_element _outactors
        (bind _asbp_controller (Utilities|Casting|CastToBP_Controller _array_element))
        (Default|GotBroadcast _asbp_controller _returnvalue)))))

(event Custom|GameCountCheck
  ;[0.15 0.15 0.15 0.5] 횟수 계산 , 무승부 처리
  (bind _outactors (Actor|GetAllActorsOfClass "/Script/Engine.PlayerController"))
  (for _array_element _outactors
    (bind _asbp_controller (Utilities|Casting|CastToBP_Controller _array_element))
    (Utilities|FlowControl|Sequence
      (:then_0
        (Development|PrintString (Utilities|String|Append (Variables|/Game/Blueprints/BP_Controller.BP_Controller_C|GetUserId _asbp_controller) " Count  : " (Utilities|String|ToString(Integer) (Variables|/Game/Blueprints/BP_Controller.BP_Controller_C|Getcount _asbp_controller))) true true "(R=0.165620,G=0.001466,B=1.000000,A=1.000000)" 5.0))
      (:then_1
        (if (Utilities|Enum|Equal(Enum) (Variables|/Game/Blueprints/BP_Controller.BP_Controller_C|GetUserId _asbp_controller) "Host")
          (Variables|Default|SetHostCount (Variables|/Game/Blueprints/BP_Controller.BP_Controller_C|Getcount _asbp_controller))
          (else
            (Variables|Default|SetGuestCount (Variables|/Game/Blueprints/BP_Controller.BP_Controller_C|Getcount _asbp_controller)))))
      (:then_2
        (if (and (<= (Variables|Default|GetHostCount) 0) (<= (Variables|Default|GetGuestCount) 0))
          (Development|PrintString "Draw" true true "(R=0.015694,G=0.170187,B=1.000000,A=1.000000)" 5.0)
          (CallFunction|ResetGame))))))

(event Custom|GotMessageFromClient
  (params (Msg :type String))
  (if (Utilities|String|Contains Msg "Host")
    (Variables|Default|SetUser "Host")
    (else
      (Variables|Default|SetUser "Geust")))
  (bind _outactors (Actor|GetAllActorsOfClass "/Script/Engine.PlayerController"))
  (for _array_element _outactors
    (bind _asbp_controller (Utilities|Casting|CastToBP_Controller _array_element))
    (Default|GotBroadcast _asbp_controller Msg)
    ;[0.15 0.15 0.15 0.5] 턴 제어
    (Default|NextTurn _asbp_controller)))

(event Custom|ResetGame
  ;[0.15 0.15 0.15 0.5] 게임 재시작
  (Variables|Default|SetEndFlag false)
  (bind _returnvalue (Class|BFRandomNumber|RandNum))
  (bind _output_get (Variables|Default|SetRandomNumber _returnvalue))
  (bind _outactors (Actor|GetAllActorsOfClass "/Script/Engine.PlayerController"))
  (for _array_element _outactors
    (bind _asbp_controller (Utilities|Casting|CastToBP_Controller _array_element))
    (Utilities|FlowControl|Sequence
      (:then_0
        (Variables|/Game/Blueprints/BP_Controller.BP_Controller_C|Setcount _asbp_controller 3)
        (Default|NextTurn _asbp_controller))
      (:then_1
        (Default|GotBroadcast _asbp_controller _output_get)))))

(event Custom|GameWinnerCheck
  (params (String :type String))
  ;[0.15 0.15 0.15 0.5] 승리 판정
  (if (Utilities|Enum|Equal(Enum) String "3S 0B 0OUT")
    (Development|PrintString (Utilities|String|Append (Variables|Default|GetUser) " Win!") true true "(R=0.165620,G=0.001466,B=1.000000,A=1.000000)" 5.0)
    (Variables|Default|SetEndFlag true)))

(event EventBeginPlay
  (bind _outactors (Actor|GetAllActorsOfClass "/Script/Engine.PlayerController"))
  (for _array_element _outactors
    (bind _asbp_controller (Utilities|Casting|CastToBP_Controller _array_element))
    ;[0.15 0.15 0.15 0.5] 난수 생성 C++ 라이브 러리
    (bind _returnvalue (Class|BFRandomNumber|RandNum))
    (bind _output_get (Variables|Default|SetRandomNumber _returnvalue))
    (Default|GotBroadcast _asbp_controller _output_get)))

(fn ConstructionScript)